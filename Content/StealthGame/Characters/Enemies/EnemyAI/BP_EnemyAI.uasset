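; Stealth-game enemy AI that patrols randomly or between target points, chases a seen player and investigates noises.
; PawnSensing sets state, and Tick uses PlayerVisible, CanMove and TargetPointMovement to choose AIMoveTo behavior.
; A montage-driven melee attack sphere-traces from the hand but stops at the player cast, applying no damage.
; UpdateWalkSpeed is empty, and the events that trigger attacks or time out sight have no callers here.
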(event `self.ReceiveBeginPlay`
  (`self.PatrolRandom`))

(event `self.ReceiveTick`
  (params (DeltaSeconds :type "Float (single-precision)"))
  (bind _bplayervisible (`self.bPlayerVisible`))
  ;[0.05234 0.1018 0.15 0.5] State
  (if (`self.bCanMove`)
    (if _bplayervisible
      (`self.ChasePlayer`)
      (elif (`self.Target Point Movement`)
        (`self.MoveToNextPatrolPoint`)
        (else
          (`self.PatrolRandom`))))
    (elif _bplayervisible
      (`self.ChasePlayer`))))

(event `self.PawnSensing.OnSeePawn`
  (params (Pawn :type "Pawn Object Reference"))
  (set `self.bPlayerVisible` true)
  (`self.ChasePlayer`))

(event `ChasePlayer`
  (if (`self.bPlayerVisible`)
    (`|AIMoveTo` self (0.0 0.0 0.0) (`GameplayStatics.GetPlayerCharacter` 0) 50.0)
    (else
      (set `self.bPlayerVisible` false))))

(event `CustomEvent`
  (params (Pawn :type "Pawn Object Reference"))
  ; See the Player
  (`|ExecutionSequence`
    (:`then_0`
      (cast `/Game/StealthGame/Core/Characters/PlayerCharacter/BP_ThirdPersonCharacterCustom` Pawn
        (:`then`
          (`KismetSystemLibrary.PrintString` "Hey! Stop right there!")
          (set `self.bPlayerVisible` true))
        (:`CastFailed`
          (set `self.bPlayerVisible` false))))
    (:`then_1`
      (`KismetSystemLibrary.RetriggerableDelay` 3.0)
      (set `self.bPlayerVisible` false))))

(event `PatrolRandom`
  (`|AIMoveTo` self (`NavigationSystemV1.K2_GetRandomReachablePointInRadius` (`self.K2_GetActorLocation`) 2000.0 null null) null 50.0))

(event `self.PawnSensing.OnHearNoise`
  (params (Instigator :type "Pawn Object Reference") (Location :type "Vector Structure (by ref)") (Volume :type "Float (single-precision)"))
  ; Hear the Object
  (`self.UpdateWalkSpeed` 200.0)
  (set `self.bCanMove` false)
  (`|AIMoveTo` self Location Instigator 80.0
    (:`OnSuccess`
      _)
    (:`OnFail`
      _))
  (`KismetSystemLibrary.Delay` 6.0)
  (set `self.bCanMove` true))

(event `CustomEvent_1`
  ; Chase Player
  (`self.UpdateWalkSpeed` 600.0)
  (set `self.bCanMove` false)
  (`|AIMoveTo` self (0.0 0.0 0.0) (`GameplayStatics.GetPlayerCharacter` 0) 80.0
    (:`OnSuccess`
      (`self.Attack`) ; new
      (`KismetSystemLibrary.Delay` 3.0)
      (set `self.bCanMove` true))))

(event `CustomEvent_2`
  ; Random Patrolling
  (`self.UpdateWalkSpeed` 50.0)
  (set `self.bCanMove` true)
  (`|AIMoveTo` self (`NavigationSystemV1.K2_GetRandomReachablePointInRadius` (`self.K2_GetActorLocation`) 1000.0 null null) null 80.0
    (:`OnSuccess`
      (`KismetSystemLibrary.Delay` 3.0)
      (set `self.bCanMove` true)
      (`self.CustomEvent_2`))))

(event `MoveToNextPatrolPoint`
  ; Patrol Points
  (`self.UpdateWalkSpeed` 200.0)
  (set `self.bCanMove` true)
  (`|AIMoveTo` self (0.0 0.0 0.0) (`|GetArrayItem` (`self.Patrol Target Points`) (`self.PatrolTargetPointIndex`)) 50.0
    (:`OnSuccess`
      (`KismetSystemLibrary.Delay` 3.0)
      (set `self.bCanMove` true)
      (`self.SetNextPatrolPointIndex`))))

(event `SetNextPatrolPointIndex`
  ; Patrol Points
  (set `self.PatrolTargetPointIndex` (mod (+ (`self.PatrolTargetPointIndex`) 1) (`KismetArrayLibrary.Array_Length` (`self.Patrol Target Points`)))))

(event `Attack`
  (bind _returnvalue (`SceneComponent.GetSocketLocation` (`self.Mesh`) "hand_r"))
  ;[0.15 0.1407 0.04319 0.5] Bonk
  (`/Engine/EditorBlueprintResources/StandardMacros.DoOnce` false :!label _label ; Only Reset Attack on miss.
    (:`Completed`
      (bind _notifyname (`|PlayMontage` (`self.Mesh`)) ; Play the AM_Attack_01
        (:`OnCompleted`
          (if (`self.bHostile`)
            (`self.ResetAttack`) ; Resets the Do Once node.
          ))
        (:`OnNotifyBegin`
          (switch `name` _notifyname ; Pick the proper attack type(standard when there is more than one type of attack)
            (:`AttackDamage`
              (`KismetSystemLibrary.PrintString` "I'm attacking!")
              (bind (_outhits _returnvalue_2) (`KismetSystemLibrary.SphereTraceMultiForObjects` _returnvalue (+ _returnvalue (* (`self.GetActorForwardVector`) (`self.Melee Trace Distance`))) (`self.Melee Trace Distance`) (`|MakeArray` "ObjectTypeQuery3" :!type "EObjectTypeQuery Enum"))) ; Trace forward from hand socket.
              (if _returnvalue_2
                (for _array_element _outhits
                  (cast `/Game/StealthGame/Core/Characters/PlayerCharacter/BP_ThirdPersonCharacterCustom` (`.HitActor` (`GameplayStatics.BreakHitResult` _array_element))))))))))))

(event `ResetAttack`
  ;[0.15 0.1407 0.04319 0.5] Bonk
  (goto _label :!via `Reset`))

(fn `UpdateWalkSpeed`
  (params (NewWalkSpeed :type "Float (double-precision)")))

(fn `UserConstructionScript`)